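; Behavior Tree task that switches the blackboard TargetLocation vector between two fixed points, then finishes successfully.
; When the key is already set, a FlipFlop alternates which point gets written on each execution.
; When it is unset, execution bypasses the FlipFlop and initializes the key through the second branch.
; An unconnected zero-vector comparison is left unused.
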(event `self.ReceiveExecute`
  (params (OwnerActor :type "Actor Object Reference"))
  (if (`BlackboardComponent.IsVectorValueSet` (`AIBlueprintHelperLibrary.GetBlackboard` OwnerActor) "TargetLocation")
    (`/Engine/EditorBlueprintResources/StandardMacros.FlipFlop`
      (:`A`
        (`BTFunctionLibrary.SetBlackboardValueAsVector` (`self.TargetLocation`) (`KismetMathLibrary.MakeVector` 0.0 0.0 200.0))
        (`self.FinishExecute` true))
      (:`B`
        (`BTFunctionLibrary.SetBlackboardValueAsVector` (`self.TargetLocation`) (`KismetMathLibrary.MakeVector` 200.0 200.0 200.0) :!label _label) ; Első TargetLocation beállítása (init)
        (`self.FinishExecute` true)))
    (else
      (goto _label))))