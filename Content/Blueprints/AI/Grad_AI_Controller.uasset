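; AI controller for the Grad pawn that starts the Grad_AI_BT behavior tree on BeginPlay.
; After launching the tree, it sets the isGradRotating blackboard key to false.
; A MoveToTestAI test event moves the pawn to a random navigable point nearby and prints a debug message, but its looping timer is disconnected, so nothing in this graph triggers it.
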(event `self.ReceiveBeginPlay`
  (`self.RunBehaviorTree` "/Game/Blueprints/AI/Grad_AI_BT.Grad_AI_BT")
  (`BlackboardComponent.SetValueAsBool` (`AIBlueprintHelperLibrary.GetBlackboard` null) "isGradRotating" false))

(event `MoveToTestAI`
  (`|AIMoveTo` (`self.K2_GetPawn`) (`NavigationSystemV1.K2_GetRandomLocationInNavigableRadius` (`self.K2_GetActorLocation` (`self.K2_GetPawn`)) 300.0 null null) null
    (:`then`
      (`KismetSystemLibrary.PrintString` "CE: MoveToTestAI"))))

(fn `UserConstructionScript`)