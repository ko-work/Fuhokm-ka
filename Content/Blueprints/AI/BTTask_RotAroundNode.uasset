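; Behavior tree task that makes the Grad AI fighter start circling the blackboard's TargetNode.
; It turns the fighter side-on to the node, then sets its RotatingMovement pivot at the negated node distance on local Y.
; Staggered delays precede a debug arrow and the rotation rate that starts the orbit.
; The task then finishes, sets IsGradRotating and clears TargetNode; a branch choosing the pivot's sign is disconnected.
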(event `self.ReceiveExecute`
  (params (OwnerActor :type "Actor Object Reference"))
  (bind _asgrad_ai_fighter (cast `/Game/Blueprints/Actors/Grad_AI_fighter` (`Controller.K2_GetPawn` (`AIBlueprintHelperLibrary.GetAIController` OwnerActor))))
  (bind _asnode_blueprint_01 (cast `/Game/Blueprints/Node_Blueprint_01` (`BTFunctionLibrary.GetBlackboardValueAsObject` (`self.TargetNode`))))
  (`|ExecutionSequence`
    (:`then_0`
      (bind _returnvalue (`Actor.K2_GetActorLocation` _asgrad_ai_fighter))
      (bind _returnvalue_2 (`Actor.K2_GetActorLocation` _asnode_blueprint_01))
      (`Actor.K2_SetActorRotation` _asgrad_ai_fighter (`KismetMathLibrary.ComposeRotators` (`KismetMathLibrary.FindLookAtRotation` _returnvalue _returnvalue_2) (struct :`Yaw` 90.0)) false)
      (`KismetSystemLibrary.Delay` 0.5))
    (:`then_1`
      (`KismetSystemLibrary.Delay` 0.2)
      (set `self.pivot_translation` (* -1 (`KismetMathLibrary.VSize` (- _returnvalue_2 _returnvalue))))
      (bind _rotatingmovement (`/Game/Blueprints/Actors/Grad_AI_fighter.RotatingMovement` _asgrad_ai_fighter))
      (set `RotatingMovementComponent.PivotTranslation` (`KismetMathLibrary.MakeVector` 0.0 (`self.pivot_translation`)) _rotatingmovement))
    (:`then_2`
      (`KismetSystemLibrary.Delay` 0.5)
      (`KismetSystemLibrary.DrawDebugArrow` _returnvalue _returnvalue_2 20.0 (struct :`R` 0.106293 :`G` 0.276042 :`B` 0.089471 :`A` 1.0) 3.0 10.0)
      (set `RotatingMovementComponent.RotationRate` (struct :`Yaw` -100.0) _rotatingmovement)
      (`self.FinishExecute` true)
      (`BTFunctionLibrary.SetBlackboardValueAsBool` (`self.isGradRotating`) true)
      (`BTFunctionLibrary.SetBlackboardValueAsObject` (`self.TargetNode`)) ; TargetNode None-ra állítása
    )))