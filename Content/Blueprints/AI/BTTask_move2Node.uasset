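; Behavior tree task that moves an AI pawn to the node stored in the TargetNode blackboard key.
; If isGradRotating is set, it first zeroes a Grad_AI_fighter's RotatingMovement rate, then snaps the pawn to face the node and sets IsGradRotating.
; AIMoveTo finishes the task on success; a failed move has no finish path.
; A separate test event moves to TargetGradNode's location and prints a counter.
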(event `self.ReceiveExecute`
  (params (OwnerActor :type "Actor Object Reference"))
  (bind _returnvalue (`Controller.K2_GetPawn` (`AIBlueprintHelperLibrary.GetAIController` OwnerActor)))
  (`self.HandleRotation` _returnvalue)
  (bind _asnode_blueprint_01 (cast `/Game/Blueprints/Actors/Node_Blueprint_01` (`BTFunctionLibrary.GetBlackboardValueAsObject` (`self.TargetNode`)))
    (:`then`
      (`Actor.K2_SetActorRotation` _returnvalue (`KismetMathLibrary.FindLookAtRotation` (`Actor.K2_GetActorLocation` _returnvalue) (`Actor.K2_GetActorLocation` _asnode_blueprint_01)) false)
      (`BTFunctionLibrary.SetBlackboardValueAsBool` (`self.isGradRotating`) true)
      (`|AIMoveTo` _returnvalue (0.0 0.0 0.0) _asnode_blueprint_01 200.0
        (:`OnSuccess`
          (`self.FinishExecute` true))))
    (:`CastFailed`
      (`self.FinishExecute` false))))

(event `MoveToNodeTestAI`
  (bind _returnvalue (`AIBlueprintHelperLibrary.GetAIController` (stale `self.ReceiveExecute` OwnerActor)))
  (bind _asnode_blueprint_01 (cast `/Game/Blueprints/Actors/Node_Blueprint_01` (`BlackboardComponent.GetValueAsObject` (`AIBlueprintHelperLibrary.GetBlackboard` _returnvalue) "TargetGradNode")))
  (`|AIMoveTo` (`Controller.K2_GetPawn` _returnvalue) (`Actor.K2_GetActorLocation` _asnode_blueprint_01) null
    (:`then`
      (`KismetSystemLibrary.PrintString` (`KismetStringLibrary.Concat_StrStr` "CE: MoveToTestAI: " (`KismetStringLibrary.Conv_IntToString` (`self.cc`))))
      (set `self.cc` (+ 1 (`self.cc`))))))

(fn `HandleRotation`
  (params (GradFighterRef :type "Actor Object Reference"))
  (if (`BlackboardComponent.GetValueAsBool` (`AIBlueprintHelperLibrary.GetBlackboard` (`AIBlueprintHelperLibrary.GetAIController` GradFighterRef)) "isGradRotating")
    (bind _asgrad_ai_fighter (cast `/Game/Blueprints/Actors/Grad_AI_fighter` GradFighterRef))
    (bind _rotatingmovement (`/Game/Blueprints/Actors/Grad_AI_fighter.RotatingMovement` _asgrad_ai_fighter))
    (if (not (== (`RotatingMovementComponent.RotationRate` _rotatingmovement) (struct)))
      (set `RotatingMovementComponent.RotationRate` (struct) _rotatingmovement))))