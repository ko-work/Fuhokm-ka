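; Behavior tree task that moves the AI-controlled pawn to the TargetLocation blackboard vector.
; On execute it runs AIMoveTo; on success it copies the target into PreviousTargetLocation and finishes successfully, with no handling for a failed move.
; A leftover MoveToTestAI event moves the pawn to random nearby navigable points and prints a counter, but its looping timer setup is disconnected.
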(event `self.ReceiveExecute`
  (params (OwnerActor :type "Actor Object Reference"))
  (bind _returnvalue (`AIBlueprintHelperLibrary.GetAIController` OwnerActor))
  (bind _returnvalue_2 (`BlackboardComponent.GetValueAsVector` (`AIBlueprintHelperLibrary.GetBlackboard` _returnvalue) "TargetLocation"))
  (`|AIMoveTo` (`Controller.K2_GetPawn` _returnvalue) _returnvalue_2 null
    (:`OnSuccess`
      (`BTFunctionLibrary.SetBlackboardValueAsVector` (`self.PreviousTargetLocation`) _returnvalue_2)
      (`self.FinishExecute` true))))

(event `MoveToTestAI`
  (bind _returnvalue (`Controller.K2_GetPawn` (`AIBlueprintHelperLibrary.GetAIController` (stale `self.ReceiveExecute` OwnerActor))))
  (`|AIMoveTo` _returnvalue (`NavigationSystemV1.K2_GetRandomLocationInNavigableRadius` (`Actor.K2_GetActorLocation` _returnvalue) 300.0 null null) null
    (:`then`
      (`KismetSystemLibrary.PrintString` (`KismetStringLibrary.Concat_StrStr` "CE: MoveToTestAI: " (`KismetStringLibrary.Conv_IntToString` (`self.cc`))))
      (set `self.cc` (+ 1 (`self.cc`))))))