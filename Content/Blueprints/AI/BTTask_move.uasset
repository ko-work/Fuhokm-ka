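; Behavior tree task that makes an AI-controlled pawn wander to random nearby navigable points.
; On execute, it starts a looping timer that repeatedly calls MoveToTestAI, which issues an AI MoveTo toward a random point around the pawn's current location.
; Each move request prints and increments a debug counter without waiting for arrival.
; The task never calls Finish Execute, and a SimpleMoveToLocation node is left unconnected.
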(event `self.ReceiveExecute`
  (params (OwnerActor :type "Actor Object Reference"))
  (`KismetSystemLibrary.K2_SetTimer` null "MoveToTestAI" 2.0 true))

(event `MoveToTestAI`
  (bind _returnvalue (`Controller.K2_GetPawn` (`AIBlueprintHelperLibrary.GetAIController` (stale `self.ReceiveExecute` OwnerActor))))
  (`|AIMoveTo` _returnvalue (`NavigationSystemV1.K2_GetRandomLocationInNavigableRadius` (`Actor.K2_GetActorLocation` _returnvalue) 300.0 null null) null
    (:`then`
      (`KismetSystemLibrary.PrintString` (`KismetStringLibrary.Concat_StrStr` "CE: MoveToTestAI: " (`KismetStringLibrary.Conv_IntToString` (`self.cc`))))
      (set `self.cc` (+ 1 (`self.cc`))))))