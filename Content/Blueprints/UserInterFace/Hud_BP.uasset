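; Player HUD Blueprint that sets up the right-click widget and draws temporary text messages on screen.
; On BeginPlay it creates the right-click widget for the first player controller, stores it and adds it to the viewport.
; Draw_Custom_01 takes the text to display and raises a flag that a Delay clears three seconds later.
; DrawHUD renders that text at enlarged scale while the flag is set.
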(event `self.ReceiveBeginPlay`
  (bind _returnvalue (`|CreateWidget` "/Game/Blueprints/UserInterFace/right_click_widget_BP.right_click_widget_BP_C" (`GameplayStatics.GetPlayerController` 0)))
  (bind _output_get (set `self.Right_Click_Widget_Var` _returnvalue))
  (`UserWidget.AddToViewport` _output_get 0))

(event `self.ReceiveDrawHUD`
  (params (SizeX :type Integer) (SizeY :type Integer))
  (if (stale `Draw_Custom_01` _output_get)
    (`self.DrawText` (`KismetTextLibrary.Conv_TextToString` (stale `Draw_Custom_01` Text_to_Display)) (struct :`A` 1) 0.0 0.0 null 3.0)))

(event `Draw_Custom_01`
  (params (Text_to_Display :type Text))
  (bind _output_get (set `self.Draw_Custom_01_bool` true))
  (`KismetSystemLibrary.Delay` 3.0)
  (set `self.Draw_Custom_01_bool` false))

(fn `UserConstructionScript`)