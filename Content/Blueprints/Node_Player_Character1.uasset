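; Player character for a node-based game, handling mouse selection and movement of Grad Fighters between nodes.
; Left click selects a node or fighter with an emissive highlight and closes the right-click menu; W spawns a fighter at the first node found.
; Right click opens that menu, or detaches the selected fighter from orbit and timeline-lerps it onto a clicked node's new orbit rotator.
; Clicked HitSpheres instead trigger test spline movement or spawn a spline.
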(event `self.ReceiveBeginPlay`
  (`|ExecutionSequence`
    (:`then_0`
      ;[1 1 1] Set HUD variable
      (bind _foundwidgets (`WidgetBlueprintLibrary.GetAllWidgetsOfClass` "/Game/Blueprints/right_click_widget_BP.right_click_widget_BP_C"))
      (set `self.Default_Hud_Widget` (`|GetArrayItem` _foundwidgets)))
    (:`then_1`
      (bind _outactors (`GameplayStatics.GetAllActorsOfClass` "/Game/Blueprints/Node_Blueprint_01.Node_Blueprint_01_C"))
      (set `self.Node_Actors_Array` _outactors))))

(event `Key|E`
  (params (Key :type "Key Structure"))
  (:`Pressed`
    (`KismetSystemLibrary.PrintString` "Hello")))

(event `Key|W`
  (params (Key :type "Key Structure"))
  ;[0.8866 1 0] Elem teremtése adott csúcsnál
  (:`Pressed`
    ;[1 1 1] Eredeti 01
    (bind _outactors (`GameplayStatics.GetAllActorsOfClass` "/Game/Blueprints/Node_Blueprint_01.Node_Blueprint_01_C"))
    (bind _output (`|GetArrayItem` _outactors))
    (`/Game/Blueprints/Node_Blueprint_01.Spawn_Grad_Fighter` _output _output)))

(event `self.ReceiveTick`
  (params (DeltaSeconds :type "Float (single-precision)"))
  ;[1 0.28 0.3199] Elem Grad Fighter másik csúcshoz küldése
  ;;[1 1 1] Másik csúcs forgatása
)

(event `Key|RightMouseButton`
  (params (Key :type "Key Structure"))
  (bind _selected_grad_var (`self.Selected_Grad_var`))
  (bind _returnvalue (`self.K2_GetActorLocation` _selected_grad_var))
  (bind _hitresult (`PlayerController.GetHitResultUnderCursorByChannel` (`GameplayStatics.GetPlayerController` 0) "TraceTypeQuery1" true))
  (bind _returnvalue_2 (`self.GetAttachParentActor` (`self.Selected_Grad_var`)))
  (bind _rootcomponent (`Actor.RootComponent` _selected_grad_var))
  ;[1 0.7802 0.2334] Csúcs teremtése az egér pozíciója mentén
  ;;[1 1 1] RMBVerticalBox megnyitása HUD Event Dispacher hívásával
  (:`Pressed`
    (if (`KismetSystemLibrary.IsValid` (`self.Selected_Grad_var`))
      ;[1 0.28 0.3199] Elem Grad Fighter másik csúcshoz küldése
      (if (`KismetSystemLibrary.IsValid` _returnvalue_2)
        (bind _asnode_grad_rotator_in_orbit (cast `/Game/Blueprints/Actors/Node_Grad_Rotator_in_Orbit` _returnvalue_2))
        (bind _output_get (set `self.Attached_Orbit_Cube_Node_Owner_Var` _asnode_grad_rotator_in_orbit))
        (`self.K2_DestroyActor` _output_get))
      (`|ExecutionSequence`
        (:`then_0`
          (`KismetSystemLibrary.PrintString` "Grad Detached")
          (bind _output_get_2 (set `self.Hit Result Hit Actor mouse` (`.HitActor` (`GameplayStatics.BreakHitResult` _hitresult))))
          (bind _asnode_blueprint_01 (cast `/Game/Blueprints/Node_Blueprint_01` _output_get_2)
            (:`then`
              (bind _returnvalue_3 (`|SpawnActorFromClass` "/Game/Blueprints/Actors/Node_Grad_Rotator_in_Orbit.Node_Grad_Rotator_in_Orbit_C" (`SceneComponent.K2_GetComponentToWorld` (`Actor.RootComponent` _asnode_blueprint_01)) "Undefined" "OverrideRootScale" null null))
              (bind (_direction _newtrack_0) (`Timeline|TL_mv_n2n` :!via `PlayFromStart`)
                (:`Update`
                  (bind _gradspringarm (`/Game/Blueprints/Actors/Node_Grad_Rotator_in_Orbit.GradSpringArm` _returnvalue_3))
                  (`self.K2_SetActorLocationAndRotation` :`self` _selected_grad_var :`NewLocation` (`KismetMathLibrary.VLerp` (`SceneComponent.K2_GetComponentLocation` _rootcomponent) (`SceneComponent.K2_GetComponentLocation` _gradspringarm) _newtrack_0)))
                (:`Finished`
                  (`SceneComponent.K2_AttachToComponent` _rootcomponent _gradspringarm "None" "SnapToTarget" "SnapToTarget" "SnapToTarget" true))))
            (:`CastFailed`
              (`KismetSystemLibrary.PrintString` (`KismetStringLibrary.Conv_VectorToString` (`.Location` (`GameplayStatics.BreakHitResult` _hitresult))))
              (`|ExecutionSequence`
                (:`then_0`
                  (bind _ashit_sphere (cast `/Game/Blueprints/Actors/HitSphere` (`self.Hit Result Hit Actor mouse`))) ; kattintható gömb a folytatás eldöntéséhez
                  (bind _ut (`/Game/Blueprints/Actors/HitSphere.ut` _ashit_sphere))
                  (if (== _ut 0)
                    (bind _outactors (`GameplayStatics.GetAllActorsOfClass` "/Game/Blueprints/Actors/spline_curve_moving_util_01.spline_curve_moving_util_01_C"))
                    (bind _asspline_curve_moving_util_01 (cast `/Game/Blueprints/Actors/spline_curve_moving_util_01` (`|GetArrayItem` _outactors)))
                    (bind (_direction_2 _newtrack_0_2) (`Timeline|spline_MU_TL` :!via `PlayFromStart`)
                      (:`Update`
                        (bind _spline_mu (`/Game/Blueprints/Actors/spline_curve_moving_util_01.Spline_MU` _asspline_curve_moving_util_01))
                        (bind _returnvalue_4 (`KismetMathLibrary.VLerp` _returnvalue (`SplineComponent.GetLocationAtSplinePoint` _spline_mu 0 "World") _newtrack_0_2))
                        (`KismetSystemLibrary.PrintString` (`KismetStringLibrary.Conv_VectorToString` _returnvalue_4))
                        (`self.K2_SetActorLocationAndRotation` :`self` _selected_grad_var :`NewLocation` _returnvalue_4))
                      (:`Finished`
                        (`KismetSystemLibrary.PrintString` "spline MU TL kész")
                        (`KismetSystemLibrary.PrintString` (`KismetStringLibrary.Concat_StrStr` "selected grad var loc2: " (`KismetStringLibrary.Conv_VectorToString` _returnvalue)))
                        (bind (_direction_3 _newtrack_0_3) (`Timeline|TL_spl_mv` :!via `PlayFromStart`)
                          (:`Update`
                            (`self.K2_SetActorLocation` (`self.Selected_Grad_var`) (`SplineComponent.GetLocationAtDistanceAlongSpline` _spline_mu (* _newtrack_0_3 (`SplineComponent.GetSplineLength` _spline_mu)) "World") false false))
                          (:`Finished`
                            (`KismetSystemLibrary.PrintString` "TL_spl_mv kész")))))
                    (elif (== _ut 1)
                      (bind _returnvalue_5 (`|SpawnActorFromClass` "/Game/Blueprints/Actors/spline_curve_moving_util_01.spline_curve_moving_util_01_C" (`self.GetTransform` _ashit_sphere) "Undefined" "OverrideRootScale" null null))
                      (bind _spline_mu_2 (`/Game/Blueprints/Actors/spline_curve_moving_util_01.Spline_MU` _returnvalue_5))
                      (bind (_returnvalue_x _returnvalue_y _returnvalue_z) (`KismetMathLibrary.BreakVector` (`SplineComponent.GetLocationAtSplinePoint` _spline_mu_2 1 "Local")))
                      (`SplineComponent.SetLocationAtSplinePoint` _spline_mu_2 1 (`KismetMathLibrary.MakeVector` _returnvalue_x (+ _returnvalue_y 200.0) _returnvalue_z) "Local" true)
                      (`SplineComponent.SetTangentAtSplinePoint` _spline_mu_2 0 (0.0 200.0 0.0) "Local" true))))))))
        (:`then_2`
          (bind _ashud_bp (cast `/Game/Blueprints/Hud_BP` (`PlayerController.GetHUD` (`GameplayStatics.GetPlayerController` 0))))
          (`/Game/Blueprints/Hud_BP.Draw_Custom_01` _ashud_bp "Grad Detached HUD")))
      (else
        (`/Game/Blueprints/right_click_widget_BP.Right_Click_Button_Event_Dispatcher_Event` (`self.Default_Hud_Widget`))))))

(event `Key|LeftMouseButton`
  (params (Key :type "Key Structure"))
  (bind _default_hud_widget (`self.Default_Hud_Widget`))
  (bind _default_hud_widget_2 (`self.Default_Hud_Widget`))
  (bind _selected_node_var (`self.Selected_Node_var`))
  (bind _hitresult (`PlayerController.GetHitResultUnderCursorByChannel` (`GameplayStatics.GetPlayerController` 0) "TraceTypeQuery1" true))
  (bind _staticmeshcomponent (`StaticMeshActor.StaticMeshComponent` _selected_node_var))
  ;[0.2384 1 0.3654] Select Node and Change Material Emissive Colour
  (:`Pressed`
    (`|ExecutionSequence`
      (:`then_0`
        (`KismetSystemLibrary.PrintString` (`KismetSystemLibrary.GetDisplayName` (`.HitActor` (`GameplayStatics.BreakHitResult` _hitresult))))
        (`|ExecutionSequence`
          (:`then_0`
            (bind _asnode_blueprint_01 (cast `/Game/Blueprints/Node_Blueprint_01` (`.HitActor` (`GameplayStatics.BreakHitResult` _hitresult)))
              (:`then`
                (set `self.Selected_Node_var` _asnode_blueprint_01)
                (if (`/Game/Blueprints/Node_Blueprint_01.Node_Selected` _asnode_blueprint_01)
                  (if (`KismetSystemLibrary.IsValid` (`self.Selected_Node_var`)) :!label _label
                    (set `/Game/Blueprints/Node_Blueprint_01.Node_Selected` false _selected_node_var)
                    (`MeshComponent.SetVectorParameterValueOnMaterials` _staticmeshcomponent "Selected_Node_Emissive_Color_3D_Vector" (0.0 0.0 0.0))
                    (set `self.Selected_Node_var` null))
                  (else
                    (`|ExecutionSequence` :!label _label_2
                      (:`then_0`
                        ;;[1 1 1] Deselect other nodes - turn off emissive color
                        (bind _outactors (`GameplayStatics.GetAllActorsOfClass` "/Game/Blueprints/Node_Blueprint_01.Node_Blueprint_01_C"))
                        (for _array_element _outactors
                          (if (`/Game/Blueprints/Node_Blueprint_01.Node_Selected` _array_element)
                            (`MeshComponent.SetVectorParameterValueOnMaterials` (`StaticMeshActor.StaticMeshComponent` _array_element) "Selected_Node_Emissive_Color_3D_Vector" (0.0 0.0 0.0))
                            (set `/Game/Blueprints/Node_Blueprint_01.Node_Selected` false _array_element))))
                      (:`then_1`
                        (set `/Game/Blueprints/Node_Blueprint_01.Node_Selected` true _selected_node_var)
                        (`MeshComponent.SetVectorParameterValueOnMaterials` _staticmeshcomponent "Selected_Node_Emissive_Color_3D_Vector" (0.0 0.4 0.02))
                        (`self.TurnOffandDeselectGradFighter`))))))
              (:`CastFailed`
                ;;[1 1 1] Bal klikk kiválasztás ledobása
                (`|ExecutionSequence`
                  (:`then_0`
                    (goto _label))
                  (:`then_1`
                    ;[1 1 1] Bal klikk Grad Fighter elem kiválasztása és szín kiemelése
                    (bind _asgrad_fighter_actor_01 (cast `/Game/Blueprints/Actors/Grad_fighter_actor_01` (`.HitActor` (`GameplayStatics.BreakHitResult` _hitresult)))
                      (:`then`
                        (if (`/Game/Blueprints/Actors/Grad_fighter_actor_01.Grad_Fighter_Selected` _asgrad_fighter_actor_01)
                          ;;[1 1 1] Mellékattintással kibocsátó szín és kiválasztás kikapcsolása
                          (if (`KismetSystemLibrary.IsValid` (`self.Selected_Grad_var`)) :!label _label_3
                            (`|ExecutionSequence`
                              (:`then_0`
                                (if (`/Game/Blueprints/right_click_widget_BP.RMBVerticalBox_Bool` _default_hud_widget_2)
                                  (`/Game/Blueprints/right_click_widget_BP.Left_Click_To_Close_Open_RMBVerticalBox_Event_Dispatcher_Event` _default_hud_widget_2)
                                  (else
                                    (set `/Game/Blueprints/Actors/Grad_fighter_actor_01.Grad_Fighter_Selected` false (`self.Selected_Grad_var`))
                                    (`MeshComponent.SetVectorParameterValueOnMaterials` (`/Game/Blueprints/Actors/Grad_fighter_actor_01.Cone` (`self.Selected_Grad_var`)) "Selected_Grad_Fighter_Emissive_Color_3D_Vector" (0.0 0.0 0.0))
                                    (set `self.Selected_Grad_var` null))))))
                          (else
                            (bind _output_get (set `self.Selected_Grad_var` _asgrad_fighter_actor_01))
                            (set `/Game/Blueprints/Actors/Grad_fighter_actor_01.Grad_Fighter_Selected` true _output_get)
                            (`MeshComponent.SetVectorParameterValueOnMaterials` (`/Game/Blueprints/Actors/Grad_fighter_actor_01.Cone` (`self.Selected_Grad_var`)) "Selected_Grad_Fighter_Emissive_Color_3D_Vector" (0.0 0.4 0.02)))))
                      (:`CastFailed`
                        (goto _label_3))))))))))
      (:`then_1`
        ;[1 0.7802 0.2334] Csúcs teremtése az egér pozíciója mentén
        ;;[1 1 1] RMBVerticalBox becsukása kívüleső bal klikk esetén
        (if (`/Game/Blueprints/right_click_widget_BP.RMBVerticalBox_Bool` _default_hud_widget)
          (`/Game/Blueprints/right_click_widget_BP.Left_Click_To_Close_Open_RMBVerticalBox_Event_Dispatcher_Event` _default_hud_widget))))))

(event `RightClickonNode`
  ;[0.2384 1 0.3654] Select Node and Change Material Emissive Colour
  ;;[1 1 1] Jobb klikk -> kiválasztás (zöld emissive) és RMBVB nyitása
  (bind _asnode_blueprint_01 (cast `/Game/Blueprints/Node_Blueprint_01` (`.HitActor` (`GameplayStatics.BreakHitResult` (`PlayerController.GetHitResultUnderCursorByChannel` (`GameplayStatics.GetPlayerController` 0) "TraceTypeQuery1" true)))))
  (set `self.Selected_Node_var` _asnode_blueprint_01)
  (goto _label_2))

(event `TurnOffandDeselectGradFighter`
  ;[1 1 1] Bal klikk Grad Fighter elem kiválasztása és szín kiemelése
  ;;[1 1 1] Mellékattintással kibocsátó szín és kiválasztás kikapcsolása
  (goto _label_3))

(event `Key|LeftMouseButton`
  (params (Key :type "Key Structure"))
  ;[0.2384 1 0.3654] Select Node and Change Material Emissive Colour
)

(event `CustomEvent`
  (bind _selected_node_var (`self.Selected_Node_var`))
  ;[0.2384 1 0.3654] Select Node and Change Material Emissive Colour
  ;;[1 1 1] Jobb klikk -> kiválasztás (zöld emissive) és RMBVB nyitása
  (bind _asnode_blueprint_01 (cast `/Game/Blueprints/Node_Blueprint_01` (`.HitActor` (`GameplayStatics.BreakHitResult` (`PlayerController.GetHitResultUnderCursorByChannel` (`GameplayStatics.GetPlayerController` 0) "TraceTypeQuery1" true)))))
  (set `self.Selected_Node_var` _asnode_blueprint_01)
  (`|ExecutionSequence`
    (:`then_0`
      ;;[1 1 1] Deselect other nodes - turn off emissive color
      (bind _outactors (`GameplayStatics.GetAllActorsOfClass` "/Game/Blueprints/Node_Blueprint_01.Node_Blueprint_01_C"))
      (for _array_element _outactors
        (if (`/Game/Blueprints/Node_Blueprint_01.Node_Selected` _array_element)
          (`MeshComponent.SetVectorParameterValueOnMaterials` (`StaticMeshActor.StaticMeshComponent` _array_element) "Selected_Node_Emissive_Color_3D_Vector" (0.0 0.0 0.0))
          (set `/Game/Blueprints/Node_Blueprint_01.Node_Selected` false _array_element))))
    (:`then_1`
      (set `/Game/Blueprints/Node_Blueprint_01.Node_Selected` true _selected_node_var)
      (`MeshComponent.SetVectorParameterValueOnMaterials` (`StaticMeshActor.StaticMeshComponent` _selected_node_var) "Selected_Node_Emissive_Color_3D_Vector" (0.0 0.4 0.02)))))

(fn `move_along_spline`)

(fn `UserConstructionScript`)