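; Node actor for the Starbattler game that registers itself with the game and can spawn Grad fighters.
; On BeginPlay it increments the game mode's node count, printing debug text, and spawns a fighter if SpawnElemDefault is set, a switch for test spawning.
; The spawn event casts the given node and creates a Grad_fighter_actor_01 at its location.
; Assigning that fighter's FirstParentNode is left disconnected and never runs.
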(event `self.ReceiveBeginPlay`
  (`|ExecutionSequence`
    (:`then_0`
      (`KismetSystemLibrary.PrintString` (`KismetSystemLibrary.GetDisplayName` self))
      (bind _ascvazer_starbattler_gamemode_bp (cast `/Game/Blueprints/cvazer_starbattler_gamemode_bp` (`GameplayStatics.GetGameMode`)))
      (bind _output_get (set `/Game/Blueprints/cvazer_starbattler_gamemode_bp.number_of_nodes` (+ (`/Game/Blueprints/cvazer_starbattler_gamemode_bp.number_of_nodes` _ascvazer_starbattler_gamemode_bp) 1) _ascvazer_starbattler_gamemode_bp))
      (`KismetSystemLibrary.PrintString` (`KismetStringLibrary.Conv_IntToString` _output_get)))
    (:`then_1`
      ;[1 1 1] First node spawn for tests - later boolean to control Elem spawning
      (if (`self.Spawn_Elem_Default`)
        (`self.Spawn_Grad_Fighter` self)))))

(event `Key|W`
  (params (Key :type "Key Structure")))

(event `Spawn_Grad_Fighter`
  (params (Current_Node :type "Object Object Reference"))
  ;[1 0.8195 0.2782] Köröző elem teremtése csúcs
  (bind _asnode_blueprint_01 (cast `/Game/Blueprints/Node_Blueprint_01` Current_Node))
  (bind _returnvalue (`SceneComponent.K2_GetComponentToWorld` (`Actor.RootComponent` _asnode_blueprint_01)))
  (bind _returnvalue_2 (`|SpawnActorFromClass` "/Game/Blueprints/Actors/Grad_fighter_actor_01.Grad_fighter_actor_01_C" (`KismetMathLibrary.MakeTransform` (`KismetMathLibrary.MakeVector` (.x (.location _returnvalue)) (.y (.location _returnvalue)) (.z (.location _returnvalue)))) "Undefined" "OverrideRootScale" null null)))

(fn `UserConstructionScript`)