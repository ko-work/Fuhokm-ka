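; Node actor for the Starbattler game that registers itself in the game mode's node count on BeginPlay.
; If SpawnElemDefault is set, it then spawns a test Grad_AI_fighter through Spawn_Grad_Fighter at a fixed location, not at the node's transform.
; Cursor hover spawns a Nyil_debug arrow at the node's transform and destroys it when the cursor leaves.
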(event `self.ReceiveBeginPlay`
  (`|ExecutionSequence`
    (:`then_0`
      (bind _ascvazer_starbattler_gamemode_bp (cast `/Game/Blueprints/cvazer_starbattler_gamemode_bp` (`GameplayStatics.GetGameMode`)))
      (set `/Game/Blueprints/cvazer_starbattler_gamemode_bp.number_of_nodes` (+ (`/Game/Blueprints/cvazer_starbattler_gamemode_bp.number_of_nodes` _ascvazer_starbattler_gamemode_bp) 1) _ascvazer_starbattler_gamemode_bp))
    (:`then_1`
      ;[1 1 1] First node spawn for tests - later boolean to control Elem spawning
      (if (`self.Spawn_Elem_Default`)
        (`self.Spawn_Grad_Fighter` self)))))

(event `Key|W`
  (params (Key :type "Key Structure")))

(event `Spawn_Grad_Fighter`
  (params (Current_Node :type "Object Object Reference"))
  ;[1 0.8195 0.2782] Köröző elem teremtése csúcs
  (bind _asnode_blueprint_01 (cast `/Game/Blueprints/Actors/Node_Blueprint_01` Current_Node))
  (`|SpawnActorFromClass` "/Game/Blueprints/Actors/Grad_AI_fighter.Grad_AI_fighter_C" (`KismetMathLibrary.MakeTransform` (0.0 0.0 200.0)) "AlwaysSpawn" "OverrideRootScale" null null))

(event `self.ReceiveActorBeginCursorOver`
  (bind _returnvalue (`|SpawnActorFromClass` "/Game/Blueprints/Actors/test_objects/nyil_debug.nyil_debug_C" (`self.GetTransform`) "Undefined" "OverrideRootScale" null null)))

(event `self.ReceiveActorEndCursorOver`
  (`self.K2_DestroyActor` (stale `self.ReceiveActorBeginCursorOver` _returnvalue)))

(fn `UserConstructionScript`)