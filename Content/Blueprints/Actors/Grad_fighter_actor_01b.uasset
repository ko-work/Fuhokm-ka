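; Fighter actor that links itself to a nearby Node_Blueprint_01 at BeginPlay.
; A sphere overlap around its Cone stores the last matching node as FirstParentNode, without comparing distances.
; Its CircleRotationSpringArm then attaches to that node's CubeToAttachSpringArms, which receives a single small yaw nudge.
; Tick is empty, and disconnected movement and rotation experiments remain in the graph.
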(event `self.ReceiveBeginPlay`
  (bind _first_parent_node (`self.First_Parent_Node`))
  (`|ExecutionSequence`
    (:`then_0`
      ;[1 1 1] Legközelebbi csúcs kiválasztása
      (bind _outactors (`KismetSystemLibrary.SphereOverlapActors` (`SceneComponent.K2_GetComponentLocation` (`self.Cone`)) 300.0 (`|MakeArray` "ObjectTypeQuery2" :!type "EObjectTypeQuery Enum")))
      (for (_array_element _array_index) _outactors
        (`KismetSystemLibrary.PrintString` (`KismetStringLibrary.Concat_StrStr` (`KismetSystemLibrary.GetDisplayName` _array_element) (`KismetStringLibrary.Conv_IntToString` _array_index) "ForAttach"))
        (bind _asnode_blueprint_01 (cast `/Game/Blueprints/Node_Blueprint_01` _array_element))
        (set `self.First_Parent_Node` _asnode_blueprint_01)))
    (:`then_1`
      ;[1 1 1] Spring Arm csatlakozás és úgy forgatás
      (if (`KismetSystemLibrary.IsValid` _first_parent_node)
        (bind _asnode_blueprint_01_2 (cast `/Game/Blueprints/Node_Blueprint_01` _first_parent_node))
        (bind _cube_toattachspringarms (`/Game/Blueprints/Node_Blueprint_01.Cube_toAttachSpringArms` _asnode_blueprint_01_2))
        (`SceneComponent.K2_AttachToComponent` (`self.CircleRotationSpringArm`) _cube_toattachspringarms "None" "KeepWorld" "KeepWorld" "KeepWorld" true)
        (`SceneComponent.K2_AddLocalRotation` _cube_toattachspringarms (struct :`Yaw` 1.0) false false)))))

(event `self.ReceiveTick`
  (params (DeltaSeconds :type "Float (single-precision)")))

(fn `UserConstructionScript`)